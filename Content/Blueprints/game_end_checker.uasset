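; Game end checker that shows the credits once every Shape_trigger in the level has found its shape.
; Each tick it gathers all Shape_trigger actors and, until the game is won, checks their FoundTheShape flags.
; When all flags are true, GameIsWon stays set, so the Credits widget is created and added to the viewport only once.
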(event EventTick
  (params (DeltaSeconds :type Float%20%28single-precision%29))
  (bind _outactors (Actor|GetAllActorsOfClass "/Game/Blueprints/shape_trigger.shape_trigger_C"))
  (if (not (Variables|Default|Getgame%20is%20won?))
    (Variables|Default|Setgame%20is%20won? true)
    (for _array_element _outactors
      (if (not (Variables|/Game/Blueprints/shape_trigger.shape_trigger_C|Getfound%20the%20shape? _array_element))
        (Variables|Default|Setgame%20is%20won? false)))
    (if (Variables|Default|Getgame%20is%20won?)
      (bind _returnvalue (UserInterface|CreateWidget "/Game/widgets/credits.credits_C"))
      (UserInterface|Viewport|AddtoViewport _returnvalue 0))))

(fn ConstructionScript)