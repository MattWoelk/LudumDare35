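; Trigger volume for a perspective shape puzzle that reacts when the first-person player stands inside it and looks in a set direction.
; Each Tick compares the overlapping character's camera rotation to the Facing component using per-axis angle tolerances.
; Holding the view for over a second calls SetMaterials to apply an unlit material to ShapePieces mesh actors.
; The timer resets when the view drifts or the player leaves.
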(event Collision|EventActorEndOverlap
  (params (OtherActor :type Actor%20Object%20Reference))
  (Utilities|Casting|CastToFirstPersonCharacter OtherActor)
  (Variables|Default|Setcontinual%20time%20in%20box 0.0))

(event EventTick
  (params (DeltaSeconds :type Float%20%28single-precision%29))
  (for _array_element (Collision|GetOverlappingActors 0 :!class /Script/Engine.Actor)
    (bind _asfirst_person_character (Utilities|Casting|CastToFirstPersonCharacter _array_element))
    (bind _desiredview (Class|CameraComponent|GetCameraView (Variables|/Game/Blueprints/FirstPersonCharacter.FirstPersonCharacter_C|GetFirstPersonCamera _asfirst_person_character) 0.0))
    (if (|issimilarrotation (.Rotation (Utilities|Struct|BreakMinimalViewInfo _desiredview)) (Transformation|GetWorldRotation (Variables|Default|Getfacing))) ; IN BOX
      (bind _output_get (Variables|Default|Setcontinual%20time%20in%20box (+ DeltaSeconds (Variables|Default|Getcontinual%20time%20in%20box))))
      (if (> _output_get 1.0)
        (CallFunction|SetMaterials "/Game/Materials/unlit2.unlit2"))
      (else
        (Variables|Default|Setcontinual%20time%20in%20box 0.0)))))

(fn ConstructionScript)

(fn SetMaterials
  (params (material :type Material%20Object%20Reference))
  (for _array_element (Variables|Default|Getshape%20pieces)
    (bind _asstatic_mesh_actor (Utilities|Casting|CastToStaticMeshActor _array_element)
      (:then
        (Rendering|Material|SetMaterial (Variables|/Script/Engine.StaticMeshActor|GetStaticMeshComponent _asstatic_mesh_actor) 0 material))
      (:CastFailed
        _))
    (return))
  (return))